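; BP_TranslucentObject is a data-generator actor that builds a randomized translucent object in its construction script.
; It sets a random static mesh from the Asset Registry folder at MeshPackagePath.
; A dynamic instance of MM_TranslucentBase then gets random opacity and roughness, plus a random HSV-based color at a configurable probability.
; It also adds itself to the TranslucentObjects actor layer; the event graph is unused.
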(event EventBeginPlay)

(event Collision|EventActorBeginOverlap
  (params (OtherActor :type Actor%20Object%20Reference)))

(event EventTick
  (params (DeltaSeconds :type Float%20%28single-precision%29)))

(fn ConstructionScript
  (CallFunction|AssignRandomMesh)
  (CallFunction|AssignRandomTranslucentMaterial)
  (Class|LayersBlueprintLibrary|AddActortoLayer self (Utilities|Struct|MakeActorLayer "TranslucentObjects")))

(fn AssignRandomMesh
  (bind _outassetdata (Class|AssetRegistry|GetAssetsbyPath (Class|AssetRegistryHelpers|GetAssetRegistry) (Variables|Default|GetMesh%20Package%20Path) false false))
  (bind _asstatic_mesh (Utilities|Casting|CastToStaticMesh (Class|AssetRegistryHelpers|GetAsset (.OutItem (Utilities|Array|Random _outassetdata)))))
  (Components|StaticMesh|SetStaticMesh (Variables|Default|GetStaticMesh) _asstatic_mesh))

(fn AssignRandomTranslucentMaterial
  (bind _returnvalue (Rendering|Material|CreateDynamicMaterialInstance (Variables|Default|GetStaticMesh) 0 "/Game/Materials/MM_TranslucentBase.MM_TranslucentBase" "None" :!class /Script/Engine.PrimitiveComponent))
  (Rendering|Material|SetScalarParameterValue _returnvalue "Opacity" (Math|Random|RandomFloatinRange 0.2 0.4) :!class /Script/Engine.MaterialInstanceDynamic)
  (Rendering|Material|SetScalarParameterValue _returnvalue "Roughness" (Math|Random|RandomFloatinRange 0.0 0.5) :!class /Script/Engine.MaterialInstanceDynamic)
  ;[1 0.6071 0.0625] Random Colour
  (if (<= (Math|Random|RandomFloat) (Variables|Default|GetProbabilityOfRandomColor))
    (Rendering|Material|SetVectorParameterValue _returnvalue "Base Color" (Class|KismetMathLibrary|HSVtoRGB (Math|Random|RandomFloat) (Math|Random|RandomFloat) 1.0 1.0) :!class /Script/Engine.MaterialInstanceDynamic)))