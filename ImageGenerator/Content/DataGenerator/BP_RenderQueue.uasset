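; BP_RenderQueue renders the LS_DataGen level sequence through Movie Render Queue, apparently for data generation.
; RenderSequence allocates a job on the queue engine subsystem, applies the MP_StillImage config, renders it and increments NumberOfRenders.
; BeginPlay binds the subsystem's render-finished callback, which broadcasts RenderEnded.
; Logic to name output files by render count exists but is disconnected, so it never runs.
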(event Custom|RenderSequence
  (bind _returnvalue (|MoviePipelineQueueEngineSubsystem))
  (bind _returnvalue_2 (Class|MoviePipelineQueueEngineSubsystem|AllocateJob _returnvalue "/Game/DataGenerator/Rendering/LS_DataGen.LS_DataGen"))
  (Class|MoviePipelineExecutorJob|SetConfiguration _returnvalue_2 "/Game/DataGenerator/Rendering/MP_StillImage.MP_StillImage")
  (Class|MoviePipelineQueueEngineSubsystem|RenderJob _returnvalue _returnvalue_2)
  (Variables|Default|SetnumberOfRenders (+ (Variables|Default|GetnumberOfRenders) 1)))

(event Custom|OnRenderFinished_Event
  (params (Results :type Movie%20Pipeline%20Output%20Data%20Structure))
  (Default|CallRenderEnded))

(event EventBeginPlay
  (EventDispatchers|AssignOnRenderFinished (|MoviePipelineQueueEngineSubsystem) (delegate Custom|OnRenderFinished_Event)))

(fn ConstructionScript)