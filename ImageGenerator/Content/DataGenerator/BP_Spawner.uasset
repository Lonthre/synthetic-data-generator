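; BP_Spawner randomly populates a scene with props and translucent objects for the data generator.
; SpawnObjects has an even chance of placing a bin (BP_Prop using the Bins mesh path) at a fixed height, followed by a short delay.
; It then spawns random, capped counts of translucent objects and props at random spawn points with horizontal jitter.
; An empty spawn point list only prints a warning.
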(event Custom|SpawnObjects
  (bind _returnvalue (Math|Random|RandomUnitVector))
  (bind _spawnpoints (Variables|Default|GetspawnPoints))
  (bind _spawnlocationoffset (Variables|Default|GetspawnLocationOffset))
  (bind _outitem (Utilities|Array|Random _spawnpoints))
  (bind (_x _y) (Math|Vector|BreakVector _returnvalue))
  (bind _returnvalue_2 (Math|Vector|MakeVector _x _y 0.0))
  (bind _returnvalue_3 (Transformation|GetActorTransform _outitem))
  (bind _location (Math|Transform|BreakTransform _returnvalue_3))
  (bind _returnvalue_4 (* _returnvalue_2 _spawnlocationoffset))
  (bind _returnvalue_5 (+ _location _returnvalue_4))
  (bind _returnvalue_6 (Math|Transform|MakeTransform _returnvalue_5))
  (if (Utilities|Array|IsNotEmpty _spawnpoints)
    (if (Math|Random|RandomBool)
      (CallFunction|SpawnBin _location)
      (Utilities|FlowControl|Delay 1.0))
    (for _index (range 1 (Math|Random|RandomIntegerinRange 1 (Variables|Default|GetnumberOfTranslucentObjects)))
      (Game|SpawnActorfromClass "/Game/DataGenerator/BP_TranslucentObject.BP_TranslucentObject_C" _returnvalue_6 "Undefined" "MultiplyWithRoot" 0 0.1 "/Game/Meshes/Import" 0))
    (for _index_2 (range 1 (Math|Random|RandomIntegerinRange 1 (Variables|Default|GetnumberOfProps)))
      (Game|SpawnActorfromClass "/Game/DataGenerator/BP_Prop.BP_Prop_C" _returnvalue_6 "Undefined" "MultiplyWithRoot" 0 "/Game/Meshes/Props" 0))
    (else
      (Development|PrintString "NO SPAWN POINTS"))))

(fn ConstructionScript)

(fn SpawnBin
  (params (InVec :type Vector))
  (bind (_x _y) (Math|Vector|BreakVector InVec))
  (Game|SpawnActorfromClass "/Game/DataGenerator/BP_Prop.BP_Prop_C" (Math|Transform|MakeTransform (Math|Vector|MakeVector _x _y 1.1e+02)) "Undefined" "MultiplyWithRoot" 0 "/Game/Meshes/Bins" 0))